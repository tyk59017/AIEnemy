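; BP_巡逻路径 is a patrol path for enemy AI that exposes points along a spline as world-space destinations.
; 获取样条线点的世界位置 returns the world location of the spline point at the current index, 当前点.
; The 递增/递减 event steps that index by 递增, flipping the step at the last and first points so traversal ping-pongs back and forth.
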(event Custom|递增/递减
  (bind _output_get (Variables|Default|Set当前点 (+ (Variables|Default|Get当前点) (Variables|Default|Get递增))))
  (if (== _output_get (- (Spline|GetNumberOfSplinePoints (Variables|Default|GetSpline)) 1))
    (Variables|Default|Set递增 -1)
    (elif (== (Variables|Default|Get当前点) 0)
      (Variables|Default|Set递增 1))))

(fn ConstructionScript)

(fn 获取样条线点的世界位置
  (return (Spline|GetLocationatSplinePoint (Variables|Default|GetSpline) (Variables|Default|Get当前点) "World")))
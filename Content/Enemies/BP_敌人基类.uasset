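; Base enemy character that pairs an AI controller (AI_敌人基类) with a damage component and a health bar widget.
; Health, healing, damage and death queries forward to BPCDamageSystem, while team, attacking and attack-token functions return fixed defaults.
; Interface functions supply the patrol path and attack/defense ranges to callers, and set walk speed by movement type.
; BeginPlay binds the component's OnDeath, and Die enables mesh physics, clears the health bar and stops AI logic.
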(event Custom|Die
  (bind _mesh (Variables|Character|GetMesh))
  (Physics|SetSimulatePhysics _mesh true)
  (Collision|SetCollisionEnabled _mesh "QueryAndPhysics")
  (UserInterface|SetWidget (Variables|Default|Get血条) 0)
  (AI|Logic|StopLogic (Variables|/Script/AIModule.AIController|GetBrainComponent (Variables|Default|GetAI%20敌人基类)) ""))

(event EventBeginPlay
  (bind _self self)
  (bind _asai_敌人基类 (Utilities|Casting|CastToAI_敌人基类 (AI|GetAIController _self)))
  (Variables|Default|SetAI%20敌人基类 _asai_敌人基类)
  (bind _returnvalue (UserInterface|CreateWidget "/Game/DamageSystem/WBP_HealthBar.WBP_HealthBar_C" 0 _self))
  (UserInterface|SetWidget (Variables|Default|Get血条) _returnvalue)
  (EventDispatchers|AssignOnDeath (Variables|Default|GetBPC_DamageSystem) (EventDispatchers|CreateEvent :!event Custom|Die)))

(fn ConstructionScript)

(fn GetCurrentHealth
  (return (Variables|/Game/DamageSystem/BPC_DamageSystem.BPC_DamageSystem_C|GetHealth (Variables|Default|GetBPC_DamageSystem))))

(fn GetMaxHealth
  (return (Variables|/Game/DamageSystem/BPC_DamageSystem.BPC_DamageSystem_C|GetMaxHealth (Variables|Default|GetBPC_DamageSystem))))

(fn GetTeamNumber
  (return 0))

(fn Heal
  (params (Amount :type Float%20%28double-precision%29))
  (bind _newhealth (Default|Heal (Variables|Default|GetBPC_DamageSystem) Amount))
  (return _newhealth))

(fn IsAttacking
  (return false))

(fn IsDead
  (return (Variables|/Game/DamageSystem/BPC_DamageSystem.BPC_DamageSystem_C|GetIsDead (Variables|Default|GetBPC_DamageSystem))))

(fn ReserveAttackToken
  (params (Amount :type Integer))
  (return false))

(fn TakeDamage
  (params (DamageInfo :type S%20Damage%20Info%20Structure) (DamageCauser :type Actor%20Object%20Reference))
  (bind _wasdamaged (Default|TakeDamage (Variables|Default|GetBPC_DamageSystem) DamageInfo DamageCauser))
  (return _wasdamaged))

(fn 巡逻路径接口
  (return (Variables|Default|Get巡逻路径)))

(fn 攻击范围和防御范围接口
  (return 1.5e+02 3.5e+02))

(fn 移动速度接口
  (params (移动类型 :type E_移动类型%20Enum :default "NewEnumerator0"))
  (bind _output_get (Variables|/Script/Engine.CharacterMovementComponent|SetMaxWalkSpeed (Variables|Character|GetCharacterMovement) (Utilities|Select :Index 移动类型 :NewEnumerator0 0.0 :NewEnumerator1 2.2e+02 :NewEnumerator2 5e+02 :NewEnumerator3 7e+02 :NewEnumerator4 1.1e+02)))
  (return _output_get))
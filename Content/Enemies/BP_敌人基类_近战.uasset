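; Melee enemy base Blueprint (敌人基类_近战) that handles sword attacks and drawing or sheathing the weapon.
; Attack montage notifies sphere-trace forward for Pawns and send damage, while BPCDamageSystem blocks interruption until the montage ends.
; Equip and unequip montage notifies attach the sword, spawned on first draw, to hand or waist sockets, with completion calling end dispatchers.
; Interface functions expose attack/defense ranges and set walk speed per movement type.
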(event EventBeginPlay
  (|CallParentFunction) ; 此节点被禁用，将不会被调用。\n从引脚连出引线来编译功能。
)

(event Event装备武器
  (bind _notifyname (Animation|Montage|PlayMontage (Variables|Character|GetMesh) "/Game/Characters/Mannequins/Animations/Manny/剑/PullOutSword_Montage.PullOutSword_Montage")
    (:OnCompleted
      (Default|CallCall装备武器结束))
    (:OnNotifyBegin
      (switch name _notifyname
        (:PullOutSword
          (Variables|Default|Get武器
            (:then
              _)
            (:else
              (bind _returnvalue (Game|SpawnActorfromClass "/Game/Weapon/BP_Weapon_Sword.BP_Weapon_Sword_C" (Transformation|GetActorTransform) "Undefined" "MultiplyWithRoot" 0 0))
              (bind _output_get (Variables|Default|Set武器 _returnvalue))))
          (Transformation|AttachComponentToComponent _output_get (Variables|Character|GetMesh) "插槽_右手近战" "SnapToTarget" "SnapToTarget" "SnapToTarget" true)
          (Variables|Default|Set是否已经装备武器 true))))))

(event Event卸下武器
  (bind _notifyname (Animation|Montage|PlayMontage (Variables|Character|GetMesh) "/Game/Characters/Mannequins/Animations/Manny/剑/InsertSword_Montage.InsertSword_Montage")
    (:OnCompleted
      (Default|CallCall卸下武器结束))
    (:OnNotifyBegin
      (switch name _notifyname
        (:InsertSword
          (Transformation|AttachComponentToComponent (Variables|Default|Get武器) (Variables|Character|GetMesh) "插槽_腰部位剑" "SnapToTarget" "SnapToTarget" "KeepRelative" true)
          (Variables|Default|Set是否已经装备武器 false))))))

(event Event攻击
  (bind _returnvalue (Transformation|GetActorLocation))
  (bind _bpc_damagesystem (Variables|Default|GetBPC_DamageSystem))
  (bind _notifyname (Animation|Montage|PlayMontage (Variables|Character|GetMesh) "/Game/Characters/Mannequins/Animations/Manny/剑/Attack1_Montage.Attack1_Montage")
    (:then
      (Variables|/Game/DamageSystem/BPC_DamageSystem.BPC_DamageSystem_C|SetIsInterruptable _bpc_damagesystem false))
    (:OnCompleted
      (Default|CallCall攻击结束 :!label _label)
      (Variables|/Game/DamageSystem/BPC_DamageSystem.BPC_DamageSystem_C|SetIsInterruptable _bpc_damagesystem true))
    (:OnInterrupted
      (goto _label))
    (:OnNotifyBegin
      (switch name _notifyname
        (:OnAttack
          (bind (_outhit _returnvalue_2) (Collision|SphereTraceForObjects _returnvalue (+ _returnvalue (* (Transformation|GetActorForwardVector) (Variables|Default|Get攻击范围))) 6e+01 (Utilities|Array|MakeArray "ObjectTypeQuery3") false 0 "ForDuration"))
          (if _returnvalue_2
            (Class|BPIDamagable|TakeDamage(Message) (.HitActor (Collision|BreakHitResult _outhit)) (Utilities|Struct|MakeS_DamageInfo (Variables|Default|Get伤害值) "NewEnumerator1" "NewEnumerator1"))))))))

(fn ConstructionScript
  (|CallParentFunction))

(fn 攻击范围和防御范围接口
  (return (Variables|Default|Get攻击范围) (Variables|Default|Get防御范围)))

(fn 移动速度接口
  (params (移动类型 :type E_移动类型%20Enum :default "NewEnumerator0"))
  (bind _output_get (Variables|/Script/Engine.CharacterMovementComponent|SetMaxWalkSpeed (Variables|Character|GetCharacterMovement) (Utilities|Select :Index 移动类型 :NewEnumerator0 0.0 :NewEnumerator1 1.8e+02 :NewEnumerator2 4e+02 :NewEnumerator3 5.5e+02 :NewEnumerator4 1e+02)))
  (return _output_get))

(fn 巡逻路径接口
  (return 0))
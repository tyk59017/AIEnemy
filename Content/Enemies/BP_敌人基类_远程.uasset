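; Ranged enemy base class that spawns a rifle on BeginPlay, attaches it to the right-hand socket and fires it at its AI target.
; Attack plays a rifle montage; on notify, a Visibility trace from weapon to the AI controller's last attack target applies damage only if nothing blocks it.
; Montage completion or interruption signals attack end.
; Interface functions supply attack and defense ranges and set walk speed by movement type.
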(event EventBeginPlay
  (|CallParentFunction)
  (CallFunction|装备武器))

(event Event攻击
  (bind _notifyname (Animation|Montage|PlayMontage (Variables|Character|GetMesh) "/Game/Characters/Mannequins/Animations/Manny/Rifle/Montage_RifleFire.Montage_RifleFire")
    (:OnCompleted
      (Default|CallCall攻击结束 :!label _label))
    (:OnInterrupted
      (goto _label))
    (:OnNotifyBegin
      (switch name _notifyname
        (:Fire
          (bind _asai_敌人基类 (Utilities|Casting|CastToAI_敌人基类 (AI|GetAIController self)))
          (bind _最后的攻击目标 (Variables|/Game/Enemies/AI/AI_敌人基类.AI_敌人基类_C|Get最后的攻击目标 _asai_敌人基类)
            (:then
              (bind _returnvalue (Collision|LineTraceByChannel (Transformation|GetActorLocation (Variables|Default|Get武器)) (Transformation|GetActorLocation _最后的攻击目标) "TraceTypeQuery1" false 0 "ForDuration"))
              (if (not _returnvalue)
                (Class|BPIDamagable|TakeDamage(Message) _最后的攻击目标 (Utilities|Struct|MakeS_DamageInfo (Variables|Default|Get伤害值) "NewEnumerator2" "NewEnumerator1"))))
            (:else)))))))

(event Event装备武器
  (bind _returnvalue (Game|SpawnActorfromClass "/Game/Weapon/BP_Weapon_Rifle.BP_Weapon_Rifle_C" (Math|Transform|MakeTransform "0, 0, 0" "0, 0, 0" "1.000000,1.000000,1.000000") "Undefined" "MultiplyWithRoot" 0 0))
  (bind _output_get (Variables|Default|Set武器 _returnvalue))
  (Transformation|AttachComponentToComponent _output_get (Variables|Character|GetMesh) "插槽_右手枪" "SnapToTarget" "SnapToTarget" "KeepRelative" true)
  (Variables|Default|Set是否已经装备武器 true))

(fn ConstructionScript
  (|CallParentFunction))

(fn 攻击范围和防御范围接口
  (return (Variables|Default|Get攻击范围) (Variables|Default|Get防御范围)))

(fn 移动速度接口
  (params (移动类型 :type E_移动类型%20Enum :default "NewEnumerator0"))
  (bind _output_get (Variables|/Script/Engine.CharacterMovementComponent|SetMaxWalkSpeed (Variables|Character|GetCharacterMovement) (Utilities|Select :Index 移动类型 :NewEnumerator0 0.0 :NewEnumerator1 2.6e+02 :NewEnumerator2 5e+02 :NewEnumerator3 7e+02 :NewEnumerator4 1.5e+02)))
  (return _output_get))
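; Attack component that gives its owning actor a hitscan bullet attack and a projectile magic attack.
; The bullet attack line-traces for Pawn objects, while the magic attack spawns a dark energy projectile aimed at a target that ignores the owner.
; Both send damage through a TakeDamage message and report it to AI Damage sense.
; Only projectile impact fires the attack-end dispatcher (攻击结束事件报告).
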(event Custom|魔法攻击
  (params (SpawnTransform :type Transform) (Target :type Actor%20Object%20Reference) (DamageInfo :type S%20Damage%20Info%20Structure))
  ;[0.15 0.15 0.15 0.5] 发射魔法攻击
  (bind _returnvalue (Game|SpawnActorfromClass "/Game/Projectiles/BP_Projectile_DarkEnergy_Alt.BP_Projectile_DarkEnergy_Alt_C" SpawnTransform "Undefined" "MultiplyWithRoot" (Components|GetOwner) 1e+03 0.0 Target false 0))
  (EventDispatchers|AssignOnProjectileImpact _returnvalue (delegate Custom|OnProjectileImpact_事件))
  (Collision|IgnoreActorwhenMoving (Variables|/Game/Projectiles/BP_Projectile_Base.BP_Projectile_Base_C|GetBoxCollision _returnvalue) (Components|GetOwner) true))

(event Custom|OnProjectileImpact_事件
  (params (OtherActor :type Actor%20Object%20Reference) (Hit :type Hit%20Result%20Structure))
  (bind _returnvalue (Components|GetOwner))
  ;[0.15 0.15 0.15 0.5] 发射魔法攻击
  (Class|BPIDamagable|TakeDamage(Message) OtherActor (stale Custom|魔法攻击 DamageInfo) _returnvalue)
  (Class|AISenseDamage|ReportDamageEvent OtherActor _returnvalue (.Amount (Utilities|Struct|BreakS_DamageInfo (stale Custom|魔法攻击 DamageInfo))) (Transformation|GetActorLocation _returnvalue) (.ImpactPoint (Collision|BreakHitResult Hit)) "None")
  (Default|Call攻击结束事件报告))

(event Custom|子弹攻击
  (params (Start :type Vector) (End :type Vector) (DamageInfo :type S%20Damage%20Info%20Structure))
  (bind _returnvalue (Components|GetOwner))
  ;[0.15 0.15 0.15 0.5] 枪类子弹攻击
  (bind (_outhit _returnvalue_2) (Collision|LineTraceForObjects Start End (Utilities|Array|MakeArray "ObjectTypeQuery3") false 0 "None"))
  (if _returnvalue_2
    (Class|BPIDamagable|TakeDamage(Message) (.HitActor (Collision|BreakHitResult _outhit)) DamageInfo _returnvalue)
    (Class|AISenseDamage|ReportDamageEvent (.HitActor (Collision|BreakHitResult _outhit)) _returnvalue (.Amount (Utilities|Struct|BreakS_DamageInfo DamageInfo)) (Transformation|GetActorLocation _returnvalue) (.ImpactPoint (Collision|BreakHitResult _outhit)) "None")))